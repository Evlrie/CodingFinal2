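; BP_MachineGun is a machine gun weapon that can be picked up, used and dropped.
; Pickup snaps it to the hand_r socket of the given skeletal mesh and turns off body collision.
; UsePrimary only prints placeholder firing text.
; Drop detaches it in world space, restores collision and simulates physics briefly before switching simulation off.
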(event `/Game/Blueprints/BPI_Itemm.Pickup`
  (params (SkeletalMesh :type "SkeletalMeshComponent Object Reference"))
  ; Pickup Function
  (`KismetSystemLibrary.PrintText` (`|FormatText` "{name} is getting picked up and attached to {mesh}." "Machine Gun" SkeletalMesh) true true (struct :`R` 1.0 :`B` 0.478632 :`A` 1.0) 6.0)
  (`self.K2_AttachToComponent` SkeletalMesh "hand_r" "SnapToTarget" "SnapToTarget" "SnapToTarget")
  (`PrimitiveComponent.SetCollisionEnabled` (`self.MachineGunBody`) "NoCollision"))

(event `/Game/Blueprints/BPI_Itemm.UsePrimary`
  (`KismetSystemLibrary.PrintText` "Pew Pew Pew"))

(event `/Game/Blueprints/BPI_Itemm.Drop`
  (`self.K2_DetachFromActor` "KeepWorld" "KeepWorld" "KeepWorld")
  (`PrimitiveComponent.SetSimulatePhysics` (`self.MachineGunBody`) true)
  (`PrimitiveComponent.SetCollisionEnabled` (`self.MachineGunBody`) "QueryAndPhysics")
  (`KismetSystemLibrary.Delay` 2.0)
  (`PrimitiveComponent.SetSimulatePhysics` (`self.MachineGunBody`) false))

(fn `UserConstructionScript`)