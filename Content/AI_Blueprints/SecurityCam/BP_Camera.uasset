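; Security camera actor that sweeps back and forth and locks onto the third-person player character when it enters its view trigger.
; A Timeline lerps the idle rotation between mirrored yaw limits, and Tick slowly interpolates the camera toward it when there is no target.
; With a target, Tick interpolates the facing vector toward the character.
; Overlap begin and end set or clear the target and switch the spotlight between red and white.
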(event `self.ReceiveBeginPlay`
  ; Camera Looks arround
  (bind (_direction _camalpha) (`Timeline|Timeline`)
    (:`Update`
      (set `self.LAST ROTATION` (`KismetMathLibrary.RLerp` (`KismetMathLibrary.MakeRotator` 0.0 (`self.CameraPitch`) (`self.CameraYaw`)) (`KismetMathLibrary.MakeRotator` 0.0 (`self.CameraPitch`) (* (`self.CameraYaw`) -1.0)) _camalpha)))))

(event `self.ReceiveTick`
  (params (DeltaSeconds :type "Float (single-precision)"))
  (bind _camera (`self.Camera`))
  (if (`self.HASTARGET`)
    (`SceneComponent.K2_SetWorldRotation` (`self.Camera`) (`KismetMathLibrary.Conv_VectorToRotator` (`KismetMathLibrary.VInterpTo` (`KismetMathLibrary.Conv_RotatorToVector` (`SceneComponent.K2_GetComponentRotation` _camera)) (`KismetMathLibrary.GetDirectionUnitVector` (`SceneComponent.K2_GetComponentLocation` _camera) (`self.K2_GetActorLocation` (`self.TARGET ACTOR`))) DeltaSeconds 5.0)) false false)
    (else
      (`SceneComponent.K2_SetRelativeRotation` (`self.Camera`) (`KismetMathLibrary.RInterpTo` (`SceneComponent.RelativeRotation` (`self.Camera`)) (`self.LAST ROTATION`) DeltaSeconds 0.5) false false))))

(event `self.view trigger.OnComponentBeginOverlap`
  (params (OverlappedComponent :type "PrimitiveComponent Object Reference") (OtherActor :type "Actor Object Reference") (OtherComp :type "PrimitiveComponent Object Reference") (OtherBodyIndex :type Integer) (bFromSweep :type Boolean) (SweepResult :type "HitResult Structure (by ref)"))
  (bind _asbp_third_person_character (cast `/Game/ThirdPerson/Blueprints/BP_ThirdPersonCharacter` OtherActor))
  (set `self.TARGET ACTOR` _asbp_third_person_character)
  (set `self.HASTARGET` true)
  (`LightComponent.SetLightColor` (`self.SpotLight`) (struct :`R` 0.918403 :`A` 1.0) true))

(event `self.view trigger.OnComponentEndOverlap`
  (params (OverlappedComponent :type "PrimitiveComponent Object Reference") (OtherActor :type "Actor Object Reference") (OtherComp :type "PrimitiveComponent Object Reference") (OtherBodyIndex :type Integer))
  (set `self.HASTARGET` false)
  (set `self.TARGET ACTOR` null)
  (`LightComponent.SetLightColor` (`self.SpotLight`) (struct :`R` 0.866087 :`G` 0.902491 :`B` 1.0 :`A` 1.0) true))

(fn `UserConstructionScript`)