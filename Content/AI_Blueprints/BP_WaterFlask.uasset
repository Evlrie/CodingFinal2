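; BP_WaterFlask is a holdable water flask item that spawns BP_HolyWater when used.
; Pickup attaches it to the supplied skeletal mesh's hand_r socket, disables flask collision and prints a debug message.
; UsePrimary spawns the holy water at the Arrow component's transform with a splash sound.
; Drop detaches the flask and re-enables collision, simulating physics for a short delay before switching it off.
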(event `self.Pickup`
  (params (SkeletalMesh :type "SkeletalMeshComponent Object Reference"))
  ; Pickup Function
  (`GameplayStatics.PlaySoundAtLocation` "/Game/AI_Blueprints/Sounds/splash1.splash1" (0.0 0.0 0.0) (struct) 1.0 1.0 0.0 null null null null)
  (`KismetSystemLibrary.PrintText` (`|FormatText` "{name} is getting picked up and attached to {mesh}." "Water Flask" SkeletalMesh) true true (struct :`R` 1.0 :`B` 0.478632 :`A` 1.0) 6.0)
  (`self.K2_AttachToComponent` SkeletalMesh "hand_r" "SnapToTarget" "SnapToTarget" "KeepRelative")
  (`PrimitiveComponent.SetCollisionEnabled` (`self.WaterFlask`) "NoCollision"))

(event `self.UsePrimary`
  (`|SpawnActorFromClass` "/Game/Blueprints/BP_HolyWater.BP_HolyWater_C" (`SceneComponent.K2_GetComponentToWorld` (`self.Arrow`)) "Undefined" "MultiplyWithRoot" null null)
  (`GameplayStatics.PlaySound2D` "/Game/AI_Blueprints/Sounds/splash1.splash1" 1.0 1.0 0.0 null null))

(event `self.Drop`
  (`self.K2_DetachFromActor` "KeepWorld" "KeepWorld")
  (`GameplayStatics.PlaySoundAtLocation` "/Engine/VREditor/Sounds/UI/Drop_Item_From_ContentBrowser.Drop_Item_From_ContentBrowser" (0.0 0.0 0.0) (struct) 1.0 1.0 0.0 null null null null)
  (`PrimitiveComponent.SetSimulatePhysics` (`self.WaterFlask`) true)
  (`PrimitiveComponent.SetCollisionEnabled` (`self.WaterFlask`) "QueryAndPhysics")
  (`KismetSystemLibrary.Delay` 2.0)
  (`PrimitiveComponent.SetSimulatePhysics` (`self.WaterFlask`) false))

(fn `UserConstructionScript`)