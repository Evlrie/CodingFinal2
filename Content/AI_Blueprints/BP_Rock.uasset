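; Throwable rock that the player picks up and drops to make noise events for AI hearing.
; Pickup attaches it to the given mesh's hand_r socket and limits collision to physics only.
; Drop detaches it, enables physics, then after a short delay applies an impulse, using the player's forward vector as target position, and reports noise.
; Its first hit on a non-player actor plays a sound and reports short-range noise instigated by the player.
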(event `self.Pickup`
  (params (SkeletalMesh :type "SkeletalMeshComponent Object Reference"))
  ; Pickup Function
  (`GameplayStatics.PlaySound2D` "/Engine/VREditor/Sounds/UI/Object_PickUp.Object_PickUp" 1.0 1.0 0.0 null null)
  (`KismetSystemLibrary.PrintText` (`|FormatText` "{name} is getting picked up and attached to {mesh}." "Water Flask" SkeletalMesh) true true (struct :`R` 1.0 :`B` 0.478632 :`A` 1.0) 6.0)
  (`self.K2_AttachToComponent` SkeletalMesh "hand_r" "SnapToTarget" "SnapToTarget" "KeepRelative")
  (`PrimitiveComponent.SetCollisionEnabled` (`self.Rock`) "PhysicsOnly")
  (`PrimitiveComponent.SetCollisionEnabled` (`self.Sphere`) "PhysicsOnly"))

(event `self.Drop`
  (bind _returnvalue (`SceneComponent.K2_GetComponentLocation` (`self.Rock`)))
  (`self.K2_DetachFromActor` "KeepWorld" "KeepWorld")
  (`PrimitiveComponent.SetSimulatePhysics` (`self.Rock`) true)
  (`PrimitiveComponent.SetSimulatePhysics` (`self.Sphere`) true)
  (`KismetSystemLibrary.Delay` 0.2)
  (`PrimitiveComponent.AddImpulse` (`self.Rock`) (* (`KismetMathLibrary.GetDirectionUnitVector` (`SceneComponent.K2_GetComponentLocation` (`self.Rock`)) (`self.GetActorForwardVector` (`GameplayStatics.GetPlayerCharacter` 0))) 1000) "None" true)
  (`PrimitiveComponent.AddImpulse` (`self.Sphere`) (* (`KismetMathLibrary.GetDirectionUnitVector` (`SceneComponent.K2_GetComponentLocation` (`self.Rock`)) (`self.GetActorForwardVector` (`GameplayStatics.GetPlayerCharacter` 0))) 1000) "None" true)
  (`GameplayStatics.SpawnSoundAtLocation` "/Engine/EngineSounds/1kSineTonePing.1kSineTonePing" _returnvalue (struct) 1.0 1.0 0.0 null null)
  (`AISense_Hearing.ReportNoiseEvent` _returnvalue 1.0 null))

(event `self.ReceiveHit`
  (params (MyComp :type "PrimitiveComponent Object Reference") (Other :type "Actor Object Reference") (OtherComp :type "PrimitiveComponent Object Reference") (bSelfMoved :type Boolean) (HitLocation :type "Vector Structure") (HitNormal :type "Vector Structure") (NormalImpulse :type "Vector Structure") (Hit :type "HitResult Structure (by ref)"))
  (bind _returnvalue (`GameplayStatics.GetPlayerCharacter` 0))
  (bind _returnvalue_2 (`self.K2_GetActorLocation`))
  (if (!= Other _returnvalue)
    (`/Engine/EditorBlueprintResources/StandardMacros.DoOnce` false
      (:`Completed`
        (`GameplayStatics.PlaySoundAtLocation` "/Game/AI_Blueprints/Sounds/RockAudioCue.RockAudioCue" _returnvalue_2 (struct) 1.0 1.0 0.0 null null null null)
        (`AISense_Hearing.ReportNoiseEvent` _returnvalue_2 1.0 _returnvalue 150.0)))))

(fn `UserConstructionScript`)