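; BP_WaterFlask is a holy water bottle item that can be picked up, dropped and used to launch holy water.
; Pickup attaches it to the hand_r socket of the given skeletal mesh and disables bottle collision.
; Drop detaches it and restores collision, simulating physics briefly before freezing it again.
; UsePrimary spawns a BP_HolyWater actor at the Player's ProjectileArrow transform, leaving the flask itself intact.
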(event `/Game/Blueprints/BPI_Item.Pickup`
  (params (`Skeletal Mesh` :type "SkeletalMeshComponent Object Reference"))
  (`KismetSystemLibrary.PrintText` "Holy waterbottle is picked up")
  (`self.K2_AttachToComponent` `Skeletal Mesh` "hand_r" "SnapToTarget" "SnapToTarget" "KeepRelative")
  (`PrimitiveComponent.SetCollisionEnabled` (`self.WaterBottle`) "NoCollision"))

(event `/Game/Blueprints/BPI_Item.Drop`
  (`self.K2_DetachFromActor` "KeepWorld" "KeepWorld")
  (`PrimitiveComponent.SetSimulatePhysics` (`self.WaterBottle`) true)
  (`PrimitiveComponent.SetCollisionEnabled` (`self.WaterBottle`) "QueryAndPhysics")
  (`KismetSystemLibrary.Delay` 2.0)
  (`PrimitiveComponent.SetSimulatePhysics` (`self.WaterBottle`) false))

(event `/Game/Blueprints/BPI_Item.UsePrimary`
  (`|SpawnActorFromClass` "/Game/Blueprints/BP_HolyWater.BP_HolyWater_C" (`SceneComponent.K2_GetComponentToWorld` (`/Game/ThirdPerson/Blueprints/BP_ThirdPersonCharacter.ProjectileArrow` (`self.Player`))) "Undefined" "MultiplyWithRoot" null null))

(fn `NewFunction`)

(fn `UserConstructionScript`)