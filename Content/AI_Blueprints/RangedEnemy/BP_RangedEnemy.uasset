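; Ranged enemy Blueprint that spawns throwable objects as its attack.
; SpawnPlate spawns the Throwable class at the ThrowableSpawn component's transform and plays a left-hook montage.
; ThrowObject is an empty event, and a disconnected older chain that launches the spawned object's sphere toward the player never runs.
; BeginPlay, Tick and the construction script add no logic, so SpawnPlate relies on an external caller.
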(event `Throw Object`
  ; Throw Rock
)

(event `SpawnPlate`
  (`|SpawnActorFromClass` "/Game/AI_Blueprints/RangedEnemy/Throwable.Throwable_C" (`SceneComponent.K2_GetComponentToWorld` (`self.ThrowableSpawn`)) "Undefined" "MultiplyWithRoot" null null)
  (`|PlayMontage` null "/Game/CloseCombatAnimSet/Animations/InPlace/Attacks/NinjaLeftHook_Montage.NinjaLeftHook_Montage"))

(fn `UserConstructionScript`
  (`parent.UserConstructionScript`))